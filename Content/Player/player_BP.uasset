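; Player Character with a constantly spinning mesh, moved by joystick and touch input, that meets falling objects and fires limited rockets.
; BeginPlay creates life bar, pause and end-menu widgets; construction loads mesh and coins from MainSave.
; Capsule overlaps branch on object type: scale-based obstacle damage, random timed-message bonuses, or saved coins.
; Depleted health pauses into the end menu; coin saves pass the coin count as UserIndex, while loads use 0.
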(event `self.ReceiveTick`
  (params (DeltaSeconds :type "Float (single-precision)"))
  ;[1 1 1] Deplacement
  (`SceneComponent.K2_AddLocalRotation` (`self.StaticMesh`) (struct :`Pitch` 0.2 :`Roll` 0.1) false false))

(event `InputTouch`
  (params (Location :type "Vector Structure") (FingerIndex :type "ETouchIndex Enum"))
  ;[1 1 1] Déplacement
  ;;[1 1 1] Input
  (:`Pressed`
    (`/Game/UltimateTouchComponents/Core/UTCMacroLibrary.UTC Touch Input Manager` Location FingerIndex :!label _label))
  (:`Released`
    (goto _label :!via `Released`))
  (:`Moved`
    (goto _label :!via `Moved`)))

(event `self.Movement Joystick.On Y Axis Changed`
  (params (Value :type "Float (single-precision)"))
  ;[1 1 1] Déplacement
  (`self.AddMovementInput` (`KismetMathLibrary.GetForwardVector` (`KismetMathLibrary.MakeRotator` 0.0 0.0 (.yaw (`self.GetControlRotation`)))) Value))

(event `self.ReceiveBeginPlay`
  (bind _returnvalue (`GameplayStatics.GetPlayerController` 0))
  ;[1 1 1] Init LifeBar / Pause Menu / End Menu
  (`|ExecutionSequence`
    (:`then_0`
      (bind _returnvalue_2 (`|CreateWidget` "/Game/Player/HUD/PauseMenu.PauseMenu_C" _returnvalue))
      (bind _output_get (set `self.PauseMenu` _returnvalue_2))
      (`Widget.SetVisibility` _output_get "Hidden")
      (`UserWidget.AddToViewport` _output_get 2)
      (bind _returnvalue_3 (`|CreateWidget` "/Game/Player/HUD/LifeBarHud.LifeBarHud_C" _returnvalue))
      (bind _output_get_2 (set `self.LifeBar` _returnvalue_3))
      (`UserWidget.AddToViewport` _output_get_2 0)
      (bind _returnvalue_4 (`|CreateWidget` "/Game/Player/HUD/EndMenu.EndMenu_C" _returnvalue))
      (bind _output_get_3 (set `self.EndMenu` _returnvalue_4))
      (`Widget.SetVisibility` _output_get_3 "Hidden")
      (`UserWidget.AddToViewport` _output_get_3 1))))

(event `self.Movement Joystick.On X Axis Changed`
  (params (Value :type "Float (single-precision)"))
  ;[1 1 1] Déplacement
  (`self.AddMovementInput` (`KismetMathLibrary.GetRightVector` (`KismetMathLibrary.MakeRotator` 0.0 0.0 (.yaw (`self.GetControlRotation`)))) Value))

(event `self.CapsuleComponent.OnComponentBeginOverlap`
  (params (OverlappedComponent :type "PrimitiveComponent Object Reference") (OtherActor :type "Actor Object Reference") (OtherComp :type "PrimitiveComponent Object Reference") (OtherBodyIndex :type Integer) (bFromSweep :type Boolean) (SweepResult :type "HitResult Structure (by ref)"))
  (bind _charactermovement (`self.CharacterMovement`))
  (bind _lifebar (`self.LifeBar`))
  (bind _lifebar_2 (`self.LifeBar`))
  ;[1 1 1] Kill FallingObject / Kill Player
  (bind _asfalling_object (cast `/Game/Blueprints/FallingObject` OtherActor))
  (switch `/Game/Blueprints/Enum/TypeObject` (`/Game/Blueprints/FallingObject.Type` _asfalling_object)
    (:`NewEnumerator0`
      (bind _output_get (set `self.Health` (- (`self.Health`) (* (`/Game/Blueprints/FallingObject.Scale` _asfalling_object) (`self.Damage`)))))
      (if (< _output_get 0.0)
        (set `self.Health` 0.0)
        (`GameplayStatics.SetGamePaused` true)
        (`Widget.SetVisibility` (`self.EndMenu`) "Visible")
        (`Widget.SetIsEnabled` (`/Game/Player/HUD/LifeBarHud.Pause` _lifebar) false)
        (`Widget.SetIsEnabled` (`/Game/Player/HUD/LifeBarHud.Rocket` _lifebar) false)
        (else
          (`GameplayStatics.SpawnEmitterAtLocation` "/Game/AdvancedMagicFX13/Particles/P_ky_explosion2.P_ky_explosion2" (`self.K2_GetActorLocation` _asfalling_object))
          (`self.K2_DestroyActor` _asfalling_object))))
    (:`NewEnumerator1`
      (switch `int` (`KismetMathLibrary.RandomIntegerInRange` 0 3)
        (:`Default`
          (`self.K2_DestroyActor` _asfalling_object))
        (:`0`
          (set `/Game/Player/HUD/LifeBarHud.BonusText` "Multiplicateur de score !" _lifebar_2)
          (set `self.Multi` (+ (`self.Multi`) 1))
          (set `/Game/Player/HUD/LifeBarHud.BonusVisible` "Visible" _lifebar_2 :!label _label_2)
          (`self.K2_DestroyActor` _asfalling_object)
          (`KismetSystemLibrary.Delay` 1.0)
          (set `/Game/Player/HUD/LifeBarHud.BonusVisible` "Hidden" _lifebar_2))
        (:`1`
          (set `/Game/Player/HUD/LifeBarHud.BonusText` "Vitesse augmenté !" _lifebar_2)
          (set `CharacterMovementComponent.MaxWalkSpeed` (+ (`CharacterMovementComponent.MaxWalkSpeed` _charactermovement) 100.0) _charactermovement)
          (goto _label_2))
        (:`2`
          (set `/Game/Player/HUD/LifeBarHud.BonusText` "Boost de vie !" _lifebar_2)
          (set `self.Health` (`self.MaxHealth`))
          (goto _label_2))
        (:`3`
          (set `/Game/Player/HUD/LifeBarHud.BonusText` "+2 Rocket !" _lifebar_2)
          (set `self.Rocket` (+ (`self.Rocket`) 2))
          (goto _label_2))))
    (:`NewEnumerator2`
      (bind _returnvalue (`GameplayStatics.LoadGameFromSlot` "MainSave"))
      (bind _assave_game_bp (cast `/Game/Blueprints/SaveGame_BP` _returnvalue))
      (bind _output_get_2 (set `/Game/Blueprints/SaveGame_BP.Coins` (+ (`/Game/Blueprints/SaveGame_BP.Coins` _assave_game_bp) 1) _assave_game_bp))
      (bind _output_get_3 (set `self.Coins` _output_get_2))
      (`GameplayStatics.SaveGameToSlot` _assave_game_bp "MainSave" _output_get_3)
      (`self.K2_DestroyActor` _asfalling_object))))

(fn `PauseGame`
  (`Widget.SetVisibility` (`self.PauseMenu`) "Visible"))

(fn `ShootRocket`
  (if (> (`self.Rocket`) 0)
    (`|SpawnActorFromClass` "/Game/Blueprints/RocketBp.RocketBp_C" (`KismetMathLibrary.MakeTransform` (`KismetMathLibrary.MakeVector` (.x (`self.K2_GetActorLocation` (`GameplayStatics.GetPlayerCharacter` 0))) (.y (`self.K2_GetActorLocation` (`GameplayStatics.GetPlayerCharacter` 0))) (- (.z (`self.K2_GetActorLocation` (`GameplayStatics.GetPlayerCharacter` 0))) 50.0))) "Undefined" "OverrideRootScale" null null)
    (set `self.Rocket` (- (`self.Rocket`) 1))))

(fn `UserConstructionScript`
  (bind _returnvalue (`GameplayStatics.LoadGameFromSlot` "MainSave"))
  (bind _assave_game_bp (cast `/Game/Blueprints/SaveGame_BP` _returnvalue)
    (:`then`
      (set `self.Coins` (`/Game/Blueprints/SaveGame_BP.Coins` _assave_game_bp))
      (`StaticMeshComponent.SetStaticMesh` (`self.StaticMesh`) (`/Game/Blueprints/SaveGame_BP.PlayerMesh` _assave_game_bp))
      (`KismetSystemLibrary.PrintString` "Hello"))
    (:`CastFailed`
      (`KismetSystemLibrary.PrintString` "CAST FAILED"))))