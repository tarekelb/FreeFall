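; RocketBp is a rocket actor that travels straight down and explodes on hitting an obstacle, clearing nearby obstacles.
; Tick spins the Rocket component and lowers the root by fixed per-frame steps, without delta-time scaling.
; When the Capsule overlaps an Obstacle-type FallingObject, the Sphere's overlaps supply the blast targets.
; Obstacles in that radius are destroyed with explosion effects, then the rocket spawns a larger explosion and destroys itself.
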(event `self.ReceiveTick`
  (params (DeltaSeconds :type "Float (single-precision)"))
  (bind _defaultsceneroot (`self.DefaultSceneRoot`))
  ;[1 1 1] Move Rocket
  (`/Engine/EditorBlueprintResources/StandardMacros.IsValid` _defaultsceneroot
    (:`Is Valid`
      (`SceneComponent.K2_AddWorldRotation` (`self.Rocket`) (`KismetMathLibrary.MakeRotator` 0.0 0.0 2.0) false false)
      (`/Engine/EditorBlueprintResources/StandardMacros.IsValid` _defaultsceneroot
        (:`Is Valid`
          (`SceneComponent.K2_AddWorldOffset` _defaultsceneroot (`KismetMathLibrary.MakeVector` 0.0 0.0 -3.0) false false))))))

(event `self.Capsule.OnComponentBeginOverlap`
  (params (OverlappedComponent :type "PrimitiveComponent Object Reference") (OtherActor :type "Actor Object Reference") (OtherComp :type "PrimitiveComponent Object Reference") (OtherBodyIndex :type Integer) (bFromSweep :type Boolean) (SweepResult :type "HitResult Structure (by ref)"))
  ;[1 1 1] Destroy Contact
  (bind _asfalling_object (cast `/Game/Blueprints/FallingObject` OtherActor))
  (switch `/Game/Blueprints/Enum/TypeObject` (`/Game/Blueprints/FallingObject.Type` _asfalling_object)
    (:`NewEnumerator0`
      (for _array_element (`PrimitiveComponent.GetOverlappingActors` (`self.Sphere`) "/Game/Blueprints/FallingObject.FallingObject_C")
        (bind _asfalling_object_2 (cast `/Game/Blueprints/FallingObject` _array_element))
        (switch `/Game/Blueprints/Enum/TypeObject` (`/Game/Blueprints/FallingObject.Type` _asfalling_object_2)
          (:`NewEnumerator0`
            (`GameplayStatics.SpawnEmitterAtLocation` "/Game/AdvancedMagicFX13/Particles/P_ky_explosion2.P_ky_explosion2" (`self.K2_GetActorLocation` _asfalling_object_2))
            (`self.K2_DestroyActor` _asfalling_object_2))))
      (`GameplayStatics.SpawnEmitterAtLocation` "/Game/AdvancedMagicFX13/Particles/P_ky_explosion3.P_ky_explosion3" (`self.K2_GetActorLocation`) (struct) (2.0 2.0 2.0))
      (`self.K2_DestroyActor` _asfalling_object)
      (`self.K2_DestroyActor`))))

(fn `UserConstructionScript`)