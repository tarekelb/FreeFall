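; FallingObject is an actor for obstacles, bonuses or coins that spin while moving along world Z.
; The construction script picks the mesh from Type: obstacles are randomly one of two meteors, with a rare table or fridge.
; Bonuses and coins get their own mesh and also show the Boost component.
; Tick applies rotation and Speed offset to the root per frame, without delta-time scaling or sweep.
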(event `self.ReceiveTick`
  (params (DeltaSeconds :type "Float (single-precision)"))
  (bind _defaultsceneroot (`self.DefaultSceneRoot`))
  ;[1 1 1] MoveActor
  (`/Engine/EditorBlueprintResources/StandardMacros.IsValid` _defaultsceneroot
    (:`Is Valid`
      (`SceneComponent.K2_AddWorldRotation` _defaultsceneroot (`KismetMathLibrary.MakeRotator` (`self.RotateX`) (`self.RotateY`) (`self.RotateZ`)) false false)
      (`/Engine/EditorBlueprintResources/StandardMacros.IsValid` _defaultsceneroot
        (:`Is Valid`
          (`SceneComponent.K2_AddWorldOffset` _defaultsceneroot (`KismetMathLibrary.MakeVector` 0.0 0.0 (`self.Speed`)) false false))))))

(fn `UserConstructionScript`
  (bind _object (`self.Object`))
  (switch `/Game/Blueprints/Enum/TypeObject` (`self.Type`)
    (:`NewEnumerator0`
      (switch `int` (`KismetMathLibrary.RandomIntegerInRange` 0 20)
        (:`Default`
          (switch `int` (`KismetMathLibrary.RandomIntegerInRange` 0 1)
            (:`Default`
              (`StaticMeshComponent.SetStaticMesh` _object "/Game/Meshes/meteor.Meteor"))
            (:`0`
              (`StaticMeshComponent.SetStaticMesh` _object "/Game/Meshes/Meteor2.Meteor2"))))
        (:`0`
          (`StaticMeshComponent.SetStaticMesh` _object "/Game/Meshes/Table.Table"))
        (:`1`
          (`StaticMeshComponent.SetStaticMesh` _object "/Game/Meshes/Fridge.Fridge"))))
    (:`NewEnumerator1`
      (`StaticMeshComponent.SetStaticMesh` _object "/Game/Meshes/Bonus.Bonus")
      (`SceneComponent.SetVisibility` (`self.Boost`) true false :!label _label))
    (:`NewEnumerator2`
      (`StaticMeshComponent.SetStaticMesh` _object "/Game/Meshes/coin.coin")
      (goto _label))))