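; My_PlayerController_BP is a player controller Blueprint that displays the menu and shop HUD widgets.
; Two events, HUD_Menu and HUD_Shop, each create their widget the first time, cache it in a variable and add it to the viewport.
; Later calls reuse the cached instance, and neither event removes the other widget or changes input mode.
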(event `HUD_Menu`
  (`/Engine/EditorBlueprintResources/StandardMacros.IsValid` (`self.Menu_HUD`)
    (:`Is Valid`
      _)
    (:`Is Not Valid`
      (bind _returnvalue (`|CreateWidget` "/Game/Map/Menu/Menu_HUD.Menu_HUD_C"))
      (bind _output_get (set `self.Menu_HUD` _returnvalue))))
  (`UserWidget.AddToViewport` _output_get 0))

(event `HUD_Shop`
  (`/Engine/EditorBlueprintResources/StandardMacros.IsValid` (`self.Shop_HUD`)
    (:`Is Valid`
      _)
    (:`Is Not Valid`
      (bind _returnvalue (`|CreateWidget` "/Game/Map/Shop/Shop_HUD.Shop_HUD_C"))
      (bind _output_get (set `self.Shop_HUD` _returnvalue))))
  (`UserWidget.AddToViewport` _output_get 0))

(fn `UserConstructionScript`)